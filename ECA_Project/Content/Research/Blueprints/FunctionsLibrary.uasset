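; Blueprint function library of helpers for a talking character driven by sentence, emotion, audio and viseme data.
; HasNewSentence checks that all five inputs are non-empty, while parsers convert strings to target and emotion enums, booleans and number lists.
; CreateEyeMovement builds a procedural, blink-like 0–1 curve from two out-of-sync periodic smoothstep pulses plus cosine jitter, using Smooth and Saturation.
; StringToListOfString parses elements as integers, despite its name.
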(fn `CreateEyeMovement`
  (params (x :type "Float (double-precision)"))
  (returns (y :type "Float (double-precision)"))
  (bind _returnvalue (`KismetMathLibrary.FMin` (`KismetMathLibrary.FMod` x 8.17) 1.0))
  (bind _returnvalue_2 (`KismetMathLibrary.FMin` (`KismetMathLibrary.FMod` x 5.12) 1.0))
  (return (`KismetMathLibrary.FMax` (`KismetMathLibrary.FMin` (+ 0.1 (* (- 1.0 0.1) (+ (`KismetMathLibrary.FMax` (- (`self.Smooth` _returnvalue_2 0.0 0.1) (`self.Smooth` _returnvalue_2 0.18 0.4)) (- (`self.Smooth` _returnvalue 0.0 0.07) (`self.Smooth` _returnvalue 0.14 0.35))) (* (`KismetMathLibrary.Cos` (`local.x`)) 0.01)))) 1.0))))

(fn `HasNewSentence`
  (params (SentenceToProcess :type "Array of String") (EmotionToProcess :type "Array of Name") (AudioToProcess :type "Array of String") (VisemeTimestampToProcess :type "Array of /Game/Research/DataStructures/Struct_Array_Float Structure") (VisemeIdToProcess :type "Array of /Game/Research/DataStructures/Struct_Array_String Structure"))
  (returns (hasSentence :type Boolean))
  (return (and (> (`KismetArrayLibrary.Array_Length` SentenceToProcess) 0) (> (`KismetArrayLibrary.Array_Length` EmotionToProcess) 0) (> (`KismetArrayLibrary.Array_Length` AudioToProcess) 0) (> (`KismetArrayLibrary.Array_Length` VisemeTimestampToProcess) 0) (> (`KismetArrayLibrary.Array_Length` VisemeIdToProcess) 0))))

(fn `Saturation`
  (params (x :type "Float (double-precision)"))
  (returns (y :type "Float (double-precision)"))
  (return (`KismetMathLibrary.FMax` -1.0 (`KismetMathLibrary.FMin` 1.0 x))))

(fn `Smooth`
  (params (x :type "Float (double-precision)") (a :type "Float (double-precision)") (b :type "Float (double-precision)"))
  (returns (y :type "Float (double-precision)"))
  (bind _y (`self.Saturation` (/ (- x a) (- b a))))
  (return (* (* _y _y) (- 3.0 (* _y 2.0)))))

(fn `StringToBool`
  (params (input :type String))
  (returns (output :type Boolean))
  (switch `string` input
    (:`True`
      (return true))
    (:`False`
      (return false))))

(fn `StringToEmotion`
  (params (input :type String))
  (returns (output :type "/Game/Research/DataStructures/Emotion Enum"))
  (switch `string` input
    (:`Emotion.ADMIRATION`
      (return (enumliteral `/Game/Research/DataStructures/Emotion` "NewEnumerator0")))
    (:`Emotion.AMUSEMENT`
      (return (enumliteral `/Game/Research/DataStructures/Emotion` "NewEnumerator1")))
    (:`Emotion.ANGER`
      (return (enumliteral `/Game/Research/DataStructures/Emotion` "NewEnumerator2")))
    (:`Emotion.ANNOYANCE`
      (return (enumliteral `/Game/Research/DataStructures/Emotion` "NewEnumerator3")))
    (:`Emotion.APPROVAL`
      (return (enumliteral `/Game/Research/DataStructures/Emotion` "NewEnumerator4")))
    (:`Emotion.CARING`
      (return (enumliteral `/Game/Research/DataStructures/Emotion` "NewEnumerator5")))
    (:`Emotion.CONFUSION`
      (return (enumliteral `/Game/Research/DataStructures/Emotion` "NewEnumerator6")))
    (:`Emotion.CURIOSITY`
      (return (enumliteral `/Game/Research/DataStructures/Emotion` "NewEnumerator7")))
    (:`Emotion.DESIRE`
      (return (enumliteral `/Game/Research/DataStructures/Emotion` "NewEnumerator8")))
    (:`Emotion.DISAPPROVAL`
      (return (enumliteral `/Game/Research/DataStructures/Emotion` "NewEnumerator9")))
    (:`Emotion.DISGUST`
      (return (enumliteral `/Game/Research/DataStructures/Emotion` "NewEnumerator10")))
    (:`Emotion.EMBARRASSMENT`
      (return (enumliteral `/Game/Research/DataStructures/Emotion` "NewEnumerator11")))
    (:`Emotion.EXCITEMENT`
      (return (enumliteral `/Game/Research/DataStructures/Emotion` "NewEnumerator12")))
    (:`Emotion.FEAR`
      (return (enumliteral `/Game/Research/DataStructures/Emotion` "NewEnumerator13")))
    (:`Emotion.GRATITUDE`
      (return (enumliteral `/Game/Research/DataStructures/Emotion` "NewEnumerator14")))
    (:`Emotion.GRIEF`
      (return (enumliteral `/Game/Research/DataStructures/Emotion` "NewEnumerator15")))
    (:`Emotion.JOY`
      (return (enumliteral `/Game/Research/DataStructures/Emotion` "NewEnumerator16")))
    (:`Emotion.LOVE`
      (return (enumliteral `/Game/Research/DataStructures/Emotion` "NewEnumerator17")))
    (:`Emotion.NERVOUSNESS`
      (return (enumliteral `/Game/Research/DataStructures/Emotion` "NewEnumerator18")))
    (:`Emotion.NEUTRAL`
      (return (enumliteral `/Game/Research/DataStructures/Emotion` "NewEnumerator19")))
    (:`Emotion.OPTIMISM`
      (return (enumliteral `/Game/Research/DataStructures/Emotion` "NewEnumerator20")))
    (:`Emotion.PRIDE`
      (return (enumliteral `/Game/Research/DataStructures/Emotion` "NewEnumerator21")))
    (:`Emotion.REALIZATION`
      (return (enumliteral `/Game/Research/DataStructures/Emotion` "NewEnumerator22")))
    (:`Emotion.RELIEF`
      (return (enumliteral `/Game/Research/DataStructures/Emotion` "NewEnumerator23")))
    (:`Emotion.REMORSE`
      (return (enumliteral `/Game/Research/DataStructures/Emotion` "NewEnumerator24")))
    (:`Emotion.SADNESS`
      (return (enumliteral `/Game/Research/DataStructures/Emotion` "NewEnumerator25")))
    (:`Emotion.SURPRISE`
      (return (enumliteral `/Game/Research/DataStructures/Emotion` "NewEnumerator26")))))

(fn `StringToListOfFloat`
  (params (input :type String))
  (returns (output :type "Array of Float (double-precision)"))
  (locals (array_float :type "Array of Float (double-precision)"))
  (for _array_element (`KismetStringLibrary.ParseIntoArray` (`KismetStringLibrary.Replace` (`KismetStringLibrary.Replace` input "[") "]") ", ")
    (`KismetArrayLibrary.Array_Add` (`local.array_float`) (`KismetStringLibrary.Conv_StringToDouble` _array_element)))
  (return (`local.array_float`)))

(fn `StringToListOfString`
  (params (input :type String))
  (returns (output :type "Array of Integer"))
  (locals (array_float :type "Array of Integer"))
  (for _array_element (`KismetStringLibrary.ParseIntoArray` (`KismetStringLibrary.Replace` (`KismetStringLibrary.Replace` (`KismetStringLibrary.Replace` input "[") "]") "'") ", ")
    (`KismetArrayLibrary.Array_Add` (`local.array_float`) (`KismetStringLibrary.Conv_StringToInt` _array_element)))
  (return (`local.array_float`)))

(fn `StringToTarget`
  (params (input :type String))
  (returns (output :type "/Game/Research/Messages/Target Enum"))
  (switch `string` input
    (:`BASIC`
      (return (enumliteral `/Game/Research/Messages/Target` "NewEnumerator3")))
    (:`MICROPHONE`
      (return (enumliteral `/Game/Research/Messages/Target` "NewEnumerator0")))
    (:`EXPRESSION`
      (return (enumliteral `/Game/Research/Messages/Target` "NewEnumerator1")))
    (:`FULL_MESSAGE`
      (return (enumliteral `/Game/Research/Messages/Target` "NewEnumerator2")))
    (:`EMOTION`
      (return (enumliteral `/Game/Research/Messages/Target` "NewEnumerator5")))))